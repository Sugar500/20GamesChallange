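; Player controller Blueprint that sets up the game's UI and handles player death.
; On BeginPlay it adds the start menu and normal play HUD to the viewport, then scans all actors for a ResetComponent.
; Each component found gets PlayerDeathEvent bound to its death delegate.
; That event pauses the game and shows a reset menu widget.
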(event `self.ReceiveBeginPlay`
  (bind _returnvalue (`|CreateWidget` "/Game/Blueprints/Widgets/BP_StartMenu.BP_StartMenu_C" self))
  (`UserWidget.AddToViewport` _returnvalue 0)
  (bind _returnvalue_2 (`|CreateWidget` "/Game/Blueprints/Widgets/NormalPlayHUD.NormalPlayHUD_C" self))
  (`UserWidget.AddToViewport` _returnvalue_2 0)
  (bind _outactors (`GameplayStatics.GetAllActorsOfClass` "/Script/Engine.Actor"))
  (for _array_element _outactors
    (bind _returnvalue_3 (`self.GetComponentByClass` _array_element "/Script/Game1_FlappyBird.ResetComponent"))
    (`/Engine/EditorBlueprintResources/StandardMacros.IsValid` _returnvalue_3
      (:`Is Valid`
        (add `ResetComponent.CallDeathDelegate` _returnvalue_3 (delegate `PlayerDeathEvent`))))))

(event `PlayerDeathEvent`
  (`GameplayStatics.SetGamePaused` true)
  (bind _returnvalue (`|CreateWidget` "/Game/Blueprints/Widgets/BP_ResetMenu.BP_ResetMenu_C" self))
  (`UserWidget.AddToViewport` _returnvalue 0))

(fn `UserConstructionScript`)